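; BP_Brain_Light_R is a visual point light that flashes when the game sequence's index changes.
; Each Tick it looks up the first BP_GameSequence_Comp actor, compares its Index to a cached copy and fires OnMiniGameEnded on a change.
; That event turns the light green for one second, then white.
; Its branch condition is fixed to true, so the red flash path never runs.
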(event `self.ReceiveTick`
  (params (DeltaSeconds :type "Float (single-precision)"))
  (bind _outactors (`GameplayStatics.GetAllActorsOfClass` "/Game/Blueprints/Games/BP_GameSequence_Comp.BP_GameSequence_Comp_C"))
  (bind _index (`/Game/Blueprints/Games/BP_GameSequence_Comp.index` (`|GetArrayItem` _outactors)))
  (if (!= (`self.Index`) _index)
    (set `self.Index` _index)
    (`self.OnMiniGameEnded`)))

(event `OnMiniGameEnded`
  (bind _outactors (`GameplayStatics.GetAllActorsOfClass` "/Game/Blueprints/Games/BP_GameSequence_Comp.BP_GameSequence_Comp_C"))
  (if true
    (`LightComponent.SetLightColor` (`self.PointLightComponent`) (struct :`G` 1.0 :`A` 1.0) true)
    (`KismetSystemLibrary.Delay` 1.0)
    (`LightComponent.SetLightColor` (`self.PointLightComponent`) (struct :`R` 1.0 :`G` 1.0 :`B` 1.0 :`A` 1.0) true)
    (else
      (`LightComponent.SetLightColor` (`self.PointLightComponent`) (struct :`R` 1.0 :`A` 1.0) true)
      (`KismetSystemLibrary.Delay` 1.0)
      (`LightComponent.SetLightColor` (`self.PointLightComponent`) (struct :`R` 1.0 :`G` 1.0 :`B` 1.0 :`A` 1.0) true))))

(fn `UserConstructionScript`)