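; BP_Brain_Light is a brain light that flashes its point light as feedback when a minigame ends.
; On BeginPlay it finds the game sequence actor; in competitive mode, a changed sequence Index is stored and triggers OnMiniGameEnded.
; That event flashes green for a second, then resets to white; its red branch is unreachable behind a constant true condition.
; The collaborative path only casts and prints a debug string.
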(event `self.ReceiveBeginPlay`
  (bind _outactors (`GameplayStatics.GetAllActorsOfClass` "/Game/Blueprints/Games/BP_GS_Parent.BP_GS_Parent_C"))
  (if (`self.iSComp`)
    (bind _output (`|GetArrayItem` _outactors))
    (bind _asbp_game_sequence_comp (cast `/Game/Blueprints/Games/BP_GameSequence_Comp` _output))
    (set `self.Out Actors` _outactors)
    (bind _index (`/Game/Blueprints/Games/BP_GameSequence_Comp.index` _asbp_game_sequence_comp))
    (if (!= (`self.Index`) _index)
      (set `self.Index` _index)
      (`self.OnMiniGameEnded`))
    (else
      (bind _asbp_game_sequence_collab (cast `/Game/Blueprints/Games/BP_GameSequence_Collab` _output))
      (`KismetSystemLibrary.PrintString` "Le laisser passer A38"))))

(event `OnMiniGameEnded`
  (bind _outactors (`GameplayStatics.GetAllActorsOfClass` "/Game/Blueprints/Games/BP_GameSequence_Comp.BP_GameSequence_Comp_C"))
  (if true
    (`LightComponent.SetLightColor` (`self.PointLightComponent`) (struct :`G` 1.0 :`A` 1.0) true)
    (`KismetSystemLibrary.Delay` 1.0)
    (`LightComponent.SetLightColor` (`self.PointLightComponent`) (struct :`R` 1.0 :`G` 1.0 :`B` 1.0 :`A` 1.0) true)
    (else
      (`LightComponent.SetLightColor` (`self.PointLightComponent`) (struct :`R` 1.0 :`A` 1.0) true)
      (`KismetSystemLibrary.Delay` 1.0)
      (`LightComponent.SetLightColor` (`self.PointLightComponent`) (struct :`R` 1.0 :`G` 1.0 :`B` 1.0 :`A` 1.0) true))))

(fn `UserConstructionScript`)