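; Stress-effect component for the VR pawn's camera that turns a triggered stress level into visual discomfort.
; Trigger and reset events set the state; ApplyStressEffect scales StressCurve by the target level, or interpolates toward it without a curve.
; ApplyPostProcess maps the current level to vignette, desaturation, exposure, FOV and random additive rotation jitter.
; The curve's time input is a difference of frame delta times, not elapsed time.
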(event `CustomEvent`
  ; Initialize the camera
  (bind _asvrpawn (cast `/Game/VRTemplate/Blueprints/VRPawn` (`self.GetOwner`)))
  (set `self.VRPawnRef` _asvrpawn)
  (`self.GetCameraView` (`Actor.GetComponentByClass` _asvrpawn "/Script/Engine.CameraComponent") 0.0))

(event `ApplyStressEffect`
  (bind _returnvalue (`GameplayStatics.GetWorldDeltaSeconds`))
  (bind _returnvalue_2 (<= (`self.CurrentStressLevel`) 0.0))
  ; Tick for stress
  (if (`self.bStressActive`)
    (set `self.Time` (- _returnvalue (`self.StressStartTime`)))
    (`/Engine/EditorBlueprintResources/StandardMacros.IsValid` (`self.StressCurve`)
      (:`Is Valid`
        (set `self.CurrentStressLevel` (`KismetMathLibrary.FClamp` (* (`CurveFloat.GetFloatValue` (`self.StressCurve`) (`self.Time`)) (`self.StressLevel`))))
        (`self.ApplyPostProcess`)
        (if _returnvalue_2
          (set `self.bStressActive` false)
          (set `self.CurrentStressLevel` 0.0)))
      (:`Is Not Valid`
        (set `self.CurrentStressLevel` (`KismetMathLibrary.FInterpTo` (`self.CurrentStressLevel`) (`self.StressLevel`) _returnvalue 2.5))
        (`self.ApplyPostProcess`)
        (if _returnvalue_2
          (set `self.bStressActive` false)
          (set `self.CurrentStressLevel` 0.0))))))

(event `TriggerStressEffect`
  (params (TargetLevel :type "Float (double-precision)" :default 0.8))
  ; TriggerStressEffect (Event)
  (set `self.StressLevel` (`KismetMathLibrary.FClamp` TargetLevel))
  (set `self.StressStartTime` (`GameplayStatics.GetWorldDeltaSeconds`))
  (set `self.bStressActive` true))

(event `ResetStressEffect`
  ; ResetStressEffect (Event)
  (set `self.StressLevel` 0.0)
  (set `self.CurrentStressLevel` 0.0)
  (set `self.bStressActive` false))

(fn `ApplyPostProcess`
  (bind _vrpawnref (`self.VRPawnRef`))
  (bind _currentstresslevel (`self.CurrentStressLevel`))
  (bind _returnvalue (* (`KismetMathLibrary.RandomFloatInRange` -0.5 0.5) (`self.CurrentStressLevel`) 1.5))
  (bind _stresseffectcameraref (`/Game/VRTemplate/Blueprints/VRPawn.StressEffectCameraRef` _vrpawnref))
  (bind _postprocesssettings (`CameraComponent.PostProcessSettings` _stresseffectcameraref))
  (`/Engine/EditorBlueprintResources/StandardMacros.IsValid` _vrpawnref
    (:`Is Valid`
      (`|ExecutionSequence`
        (:`then_0`
          (setmembers `PostProcessSettings` :`StructRef` _postprocesssettings :`VignetteIntensity` (`KismetMathLibrary.Lerp` 0.2 1.0 (`self.CurrentStressLevel`))) ; VignetteIntensity
        )
        (:`then_1`
          (setmembers `PostProcessSettings` :`StructRef` _postprocesssettings :`ColorSaturation` (`KismetMathLibrary.MakeVector4` (`KismetMathLibrary.Lerp` 1.0 0.4 _currentstresslevel) (`KismetMathLibrary.Lerp` 1.0 0.4 _currentstresslevel) (`KismetMathLibrary.Lerp` 1.0 0.4 _currentstresslevel) 1.0)) ; ColorSaturation
        )
        (:`then_2`
          (setmembers `PostProcessSettings` :`StructRef` _postprocesssettings :`AutoExposureBias` (`KismetMathLibrary.Lerp` 1.0 0.6 _currentstresslevel)) ; AutoExposureBias
        )
        (:`then_3`
          (`self.K2_AddLocalRotation` _stresseffectcameraref (`KismetMathLibrary.MakeRotator` 0.0 _returnvalue _returnvalue) false false) ; Tremblement
        )
        (:`then_4`
          (`self.SetFieldOfView` _stresseffectcameraref (`KismetMathLibrary.Lerp` 90.0 100.0 (`self.CurrentStressLevel`))) ; Field of View
        )))))