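; BP_ButtonInteraction is a VR answer button that plays a right- or wrong-answer sound based on IsRightButton.
; Hand controller overlap highlights it and calls Interact, then, if unlocked, checks hand proximity and the opposite side's hover flag.
; A valid press runs a lock-and-timeline animation, whose location lerp has a fixed zero alpha, and sets LinkedFunction to the empty NextPhase.
; Hover events maintain the left and right flags for VRInteractor-tagged hands.
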(event `self.Collision.OnComponentBeginOverlap`
  (params (OverlappedComponent :type "PrimitiveComponent Object Reference") (OtherActor :type "Actor Object Reference") (OtherComp :type "PrimitiveComponent Object Reference") (OtherBodyIndex :type Integer) (bFromSweep :type Boolean) (SweepResult :type "HitResult Structure (by ref)"))
  ; Interaction of buttons depending on inputs
  (cast `/Game/Blueprints/Logic/BP_HandVRController` OtherActor)
  (switch `EControllerHand` "Right"
    (:`Left`
      (`|ExecutionSequence`
        (:`then_0`
          (bind _returnvalue (`GameplayStatics.GetActorOfClass` "/Game/Blueprints/Logic/BP_VRCharacter.BP_VRCharacter_C"))
          (`self.Highlight` true)
          (bind _handlocation (`/Game/Blueprints/Logic/BP_HandVRController.HandLocation` (stale _returnvalue_2)))
          (`self.Interact` "NewEnumerator1" (`/Game/Blueprints/Logic/BP_VRCharacter.LeftHandController` _returnvalue) _handlocation)
          (if (not (`self.bIsLocked`))
            (bind _ishandclosetoobject (`self.IsHandCloseEnough` _handlocation (`SceneComponent.K2_GetComponentLocation` (`self.StaticMeshComponent`)) 4.0))
            (if (and _ishandclosetoobject (`self.bIsHoveredRight`))
              (`self.AnimateButtonInteraction`)
              (`self.ReturnValue`))))
        (:`then_1`
          (bind _returnvalue_2 (`GameplayStatics.GetActorOfClass` "/Game/Blueprints/Logic/BP_HandVRController.BP_HandVRController_C")))))
    (:`Right`
      (`|ExecutionSequence`
        (:`then_0`
          (bind _returnvalue_3 (`GameplayStatics.GetActorOfClass` "/Game/Blueprints/Logic/BP_VRCharacter.BP_VRCharacter_C"))
          (`self.Highlight` true)
          (bind _handlocation_2 (`/Game/Blueprints/Logic/BP_HandVRController.HandLocation` (stale _returnvalue_4)))
          (`self.Interact` "NewEnumerator1" (`/Game/Blueprints/Logic/BP_VRCharacter.RightHandController` _returnvalue_3) _handlocation_2)
          (if (not (`self.bIsLocked`))
            (bind _ishandclosetoobject_2 (`self.IsHandCloseEnough` _handlocation_2 (`SceneComponent.K2_GetComponentLocation` (`self.StaticMeshComponent`)) 4.0))
            (if (and (`self.bIsHoveredLeft`) _ishandclosetoobject_2)
              (`self.AnimateButtonInteraction`)
              (`self.ReturnValue`))))
        (:`then_1`
          (bind _returnvalue_4 (`GameplayStatics.GetActorOfClass` "/Game/Blueprints/Logic/BP_HandVRController.BP_HandVRController_C")))))))

(event `ReturnValue`
  ; Game Logic
  (if (`self.IsRightButton`)
    (`GameplayStatics.PlaySound2D` "/Game/Audio/Son_bonne_reponse.Son_bonne_reponse" 1.0 1.0 0.0 null null)
    (set `self.Loop` false)
    (else
      (`GameplayStatics.PlaySound2D` "/Game/Audio/Son_mauvaise_reponse.Son_mauvaise_reponse" 1.0 1.0 0.0 null null)
      (set `self.Loop` false))))

(event `AnimationPress`
  (bind _startlocation (`self.StartLocation`))
  ; Animation of pressed button
  (set `self.bIsLocked` true)
  (`Timeline|TL_ButtonPress` :!label _label
    (:`Update`
      (`SceneComponent.K2_SetRelativeLocation` (`self.StaticMeshComponent`) (`KismetMathLibrary.VLerp` _startlocation (- _startlocation (`KismetMathLibrary.MakeVector` 0.0 0.0 (`self.PressedOffset`)))) false false)
      (`KismetSystemLibrary.Delay` 0.5)
      (goto _label :!via `Reverse`))
    (:`Finished`
      (`KismetSystemLibrary.Delay` 0.5)
      (set `self.bIsLocked` false)
      (goto _label :!via `Stop`))))

(event `self.OnHoverBegin`
  (params (HandController :type "/Game/Blueprints/Logic/BP_HandVRController Object Reference"))
  ; VRHand hovering the button
  (bind _output_get (set `self.HoveredBy` HandController))
  (if (`self.ActorHasTag` _output_get "VRInteractor")
    (switch `EControllerHand` "Right"
      (:`Left`
        (set `self.bIsHoveredLeft` true))
      (:`Right`
        (set `self.bIsHoveredRight` true)))))

(event `self.OnHoverEnd`
  (params (HandController :type "/Game/Blueprints/Logic/BP_HandVRController Object Reference"))
  ; VRHand hovering the button
  (bind _output_get (set `self.HoveredBy` HandController))
  (if (`self.ActorHasTag` _output_get "VRInteractor")
    (switch `EControllerHand` "Right"
      (:`Left`
        (set `self.bIsHoveredLeft` false))
      (:`Right`
        (set `self.bIsHoveredRight` false)))))

(fn `AnimateButtonInteraction`
  (`self.AnimationPress`)
  (set `self.LinkedFunction` "NextPhase"))

(fn `NextPhase`)

(fn `UserConstructionScript`
  (`parent.UserConstructionScript`))