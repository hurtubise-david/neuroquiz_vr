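; VR grabbable object that attaches to a hand on overlap and detaches when the overlap ends.
; Collision accepts sphere components, branches by left or right hand, and calls Grab with that hand's controller and interaction origin.
; If CanBeGrabbed, it attaches with location snapped and tracks IsHeld and HeldByHand; end overlap clears both.
; The motion controller casts supplying the attach parents sit on unexecuted chains.
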(event OnComponentBeginOverlap(Collision)
  (params (OverlappedComponent :type Primitive%20Component%20Object%20Reference) (OtherActor :type Actor%20Object%20Reference) (OtherComp :type Primitive%20Component%20Object%20Reference) (OtherBodyIndex :type Integer) (bFromSweep :type Boolean) (SweepResult :type Hit%20Result%20Structure%20%28by%20ref%29))
  ;[0.15 0.15 0.15 0.5] Logic of grabbing objects with each hand
  (Utilities|Casting|CastToSphereComponent OtherComp)
  (bind _asbp_hand_vrcontroller (Utilities|Casting|CastTo OtherActor))
  (bind _output_get (Variables|Default|SetHeldByHand _asbp_hand_vrcontroller))
  (switch Utilities|FlowControl|Switch|SwitchonEControllerHand "Right"
    (:Left
      (bind _returnvalue (Actor|GetActorOfClass 0))
      (Utilities|IsValid (Variables|Default|GetLeftHandController _returnvalue)
        (:Is%20Valid
          (bind _returnvalue_2 (Actor|GetActorOfClass 0))
          (bind _interactionorigin (CallFunction|GetInteractionOrigin _returnvalue_2 "Left"))
          (Default|Grab _output_get "NewEnumerator2" (Variables|Default|GetLeftHandController _returnvalue) (Transformation|GetWorldLocation _interactionorigin))
          (if (Variables|Default|GetbCanBeGrabbed)
            (bind _returnvalue_3 (Transformation|AttachComponentToComponent (stale _asmotion_controller_component) "None" "SnapToTarget" "KeepWorld" "KeepWorld" true))
            (Variables|Default|SetbIsHeld _returnvalue_3)
            (Variables|Default|SetHeldByHand (Variables|Default|GetLeftHandController _returnvalue))))))
    (:Right
      (bind _returnvalue_4 (Actor|GetActorOfClass 0))
      (Utilities|IsValid (Variables|Default|GetRightHandController _returnvalue_4)
        (:Is%20Valid
          (bind _returnvalue_5 (Actor|GetActorOfClass 0))
          (bind _interactionorigin_2 (CallFunction|GetInteractionOrigin _returnvalue_5 "Right"))
          (Default|Grab _output_get "NewEnumerator2" (Variables|Default|GetRightHandController _returnvalue_4) (Transformation|GetWorldLocation _interactionorigin_2))
          (if (Variables|Default|GetbCanBeGrabbed)
            (bind _returnvalue_6 (Transformation|AttachComponentToComponent (stale _asmotion_controller_component) "None" "SnapToTarget" "KeepWorld" "KeepWorld" true))
            (Variables|Default|SetbIsHeld _returnvalue_6)
            (Variables|Default|SetHeldByHand (Variables|Default|GetRightHandController _returnvalue_4))))))))

(event OnComponentEndOverlap(Collision)
  (params (OverlappedComponent :type Primitive%20Component%20Object%20Reference) (OtherActor :type Actor%20Object%20Reference) (OtherComp :type Primitive%20Component%20Object%20Reference) (OtherBodyIndex :type Integer))
  ;[0.15 0.15 0.15 0.5] Logic of grabbing objects with each hand
  (Utilities|Casting|CastToSphereComponent OtherComp)
  (bind _asbp_hand_vrcontroller (Utilities|Casting|CastTo OtherActor))
  (bind _output_get (Variables|Default|SetHeldByHand _asbp_hand_vrcontroller))
  (switch Utilities|FlowControl|Switch|SwitchonEControllerHand "Right"
    (:Left
      (Utilities|IsValid (Variables|Default|GetLeftHandController (stale OnComponentBeginOverlap(Collision) _returnvalue))
        (:Is%20Valid
          (Default|Grab _output_get "NewEnumerator0" (Variables|Default|GetLeftHandController (stale OnComponentBeginOverlap(Collision) _returnvalue)) (Transformation|GetWorldLocation (stale OnComponentBeginOverlap(Collision) _interactionorigin)))
          (Transformation|DetachFromActor "KeepWorld" "KeepWorld" "KeepWorld")
          (Variables|Default|SetbIsHeld false)
          (Variables|Default|SetHeldByHand 0))))
    (:Right
      (Utilities|IsValid (Variables|Default|GetRightHandController (stale OnComponentBeginOverlap(Collision) _returnvalue_4))
        (:Is%20Valid
          (Default|Grab _output_get "NewEnumerator0" (Variables|Default|GetRightHandController (stale OnComponentBeginOverlap(Collision) _returnvalue_4)) (Transformation|GetWorldLocation (stale OnComponentBeginOverlap(Collision) _interactionorigin_2)))
          (Transformation|DetachFromActor "KeepWorld" "KeepWorld" "KeepWorld")
          (Variables|Default|SetbIsHeld false)
          (Variables|Default|SetHeldByHand 0))))))

(fn ConstructionScript
  (|CallParentFunction))