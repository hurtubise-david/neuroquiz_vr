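; BP_InteractableBase is a base Blueprint for objects that hand controllers can hover, grab and interact with.
; Its hover, Interact and Grab events are empty stubs, and BeginPlay initializes HoveredBy to the right hand controller of a found actor.
; Highlight toggles HighlightMesh visibility and its outline overlay material, using IsHighlighted to skip redundant calls.
; IsHandCloseEnough provides a distance-threshold check between hand and target locations.
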(event `OnHoverBegin`
  (params (HandController :type "Object Object Reference")))

(event `OnHoverEnd`
  (params (HandController :type "Object Object Reference")))

(event `Interact`
  (params (`Interaction Type` :type "/Game/Blueprints/Logic/ENUM_InteractionType Enum" :default "NewEnumerator0") (HandController :type "Object Object Reference") (HandLocation :type "Vector Structure")))

(event `Grab`
  (params (InteractionType :type "/Game/Blueprints/Logic/ENUM_InteractionType Enum" :default "NewEnumerator2") (HandController :type "Object Object Reference") (HandLocation :type "Vector Structure")))

(event `self.ReceiveBeginPlay`
  (bind _returnvalue (`GameplayStatics.GetActorOfClass` null))
  (set `self.HoveredBy` (`/Game/Blueprints/Logic/BP_InteractableBase.RightHandController` _returnvalue)))

(fn `Highlight`
  (params (bEnable :type Boolean))
  (if (== bEnable (`self.bIsHighlighted`))
    _
    (elif bEnable
      (`SceneComponent.SetVisibility` (`self.HighlightMesh`) true false)
      (`MeshComponent.SetOverlayMaterial` (`self.HighlightMesh`) "/Game/Materials/Outline_Material.Outline_Material")
      (set `self.bIsHighlighted` true)
      (else
        (`SceneComponent.SetVisibility` (`self.HighlightMesh`) false false)
        (`MeshComponent.SetOverlayMaterial` (`self.HighlightMesh`) null)
        (set `self.bIsHighlighted` false)))))

(fn `IsHandCloseEnough`
  (params (HandLocation :type "Vector Structure") (TargetLocation :type "Vector Structure") (Threshold :type "Float (double-precision)"))
  (returns (IsHandCloseToObject :type Boolean))
  (return (< (`KismetMathLibrary.VSize` (- HandLocation TargetLocation)) Threshold)))

(fn `UserConstructionScript`)