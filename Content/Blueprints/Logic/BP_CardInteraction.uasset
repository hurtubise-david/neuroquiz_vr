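; Card interaction Blueprint meant to twist a card a quarter turn either way depending on the VR hand.
; BeginPlay attaches the mesh to FlipPivot, whose yaw TwistCard drives through a Timeline, saving the target angle on finish.
; The Lerp alpha is fixed at zero, so the twist does not animate toward its target.
; The hand-tag check, highlight and left/right targeting are unwired and never run.
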(event `self.ReceiveBeginPlay`
  ; Interaction of cards with each hand (to be ajusted)
  (`SceneComponent.K2_AttachToComponent` (`self.StaticMeshComponent`) (`self.FlipPivot`) "None" "KeepWorld" "KeepWorld" "KeepWorld" true))

(event `StartTwist`
  (bind (_returnvalue_roll _returnvalue_pitch _returnvalue_yaw) (`KismetMathLibrary.BreakRotator` (`KismetMathLibrary.MakeRotator` 0.0 0.0 (`KismetMathLibrary.Lerp` (`self.TwistRotation`) (`self.TargetTwistAngle`)))))
  ; Timeline for twisting cards
  (`Timeline|Timeline` :!via `PlayFromStart`
    (:`Update`
      (`SceneComponent.K2_SetRelativeRotation` (`self.FlipPivot`) (`KismetMathLibrary.MakeRotator` 0.0 0.0 _returnvalue_yaw) false false))
    (:`Finished`
      (set `self.TwistRotation` (`self.TargetTwistAngle`)))))

(fn `TwistCard`
  (`self.StartTwist`))

(fn `UserConstructionScript`)