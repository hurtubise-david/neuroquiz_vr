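; Memory-list minigame Blueprint that plays narrated audio, then has the player pick one of four answer sets in a widget.
; StartEvent plays the question and fills WBP_Memory; chained audio-finished callbacks play a second clip, then reveal the answers.
; The chosen index is compared to GoodAnswer and reported through CallOnMinigameEnd.
; A 30-second timeout from the second clip's start reports failure, with no check for an earlier answer.
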(event `self.StartEvent`
  (bind _returnvalue (`GameplayStatics.SpawnSoundAtLocation` (`self.QuestionNarration`) (-20.0 400.0 30.0) (struct) 1.0 1.0 0.0 null null))
  (add `AudioComponent.OnAudioFinished` _returnvalue (delegate `QuestionFinished`))
  (`KismetSystemLibrary.Delay` 0.01)
  (`WidgetComponent.SetWindowVisibility` (`self.Widget`) "Visible")
  (bind _aswbp_memory (cast `/Game/UI/WBP_Memory` (`WidgetComponent.GetUserWidgetObject` (`self.Widget`))))
  (if (`KismetSystemLibrary.IsValid` _aswbp_memory)
    (bind _output_get (set `self.WBP_mem` _aswbp_memory))
    (`/Game/UI/WBP_Memory.SetAnswers` _output_get (`self.AnswerSet_1`) (`self.AnswerSet_2`) (`self.AnswerSet_3`) (`self.AnswerSet_4`))))

(event `QuestionFinished`
  (bind _returnvalue (`GameplayStatics.SpawnSoundAtLocation` (`self.Partie2`) (-20.0 400.0 30.0) (struct) 1.0 1.0 0.0 null null))
  (add `AudioComponent.OnAudioFinished` _returnvalue (delegate `AudioFinished`))
  ; Après 30 sec auto perd si il est pas dejà fini
  (`KismetSystemLibrary.Delay` 30.0)
  (`/Game/UI/WBP_Memory.HideAll` (`self.WBP_mem`))
  (`WidgetComponent.SetWindowVisibility` (`self.Widget`) "SelfHitTestInvisible")
  (`self.OnMinigameEnd` false))

(event `AudioFinished`
  (bind _wbp_mem (`self.WBP_mem`))
  (`/Game/UI/WBP_Memory.DisplayAnswers` _wbp_mem)
  (add `/Game/UI/WBP_Memory.OnAnswerChosen` _wbp_mem (delegate `AnswerChosen`)))

(event `AnswerChosen`
  (params (AnswerIndex :type Integer))
  (`KismetSystemLibrary.Delay` 0.1)
  (`/Game/UI/WBP_Memory.HideAll` (`self.WBP_mem`))
  (`WidgetComponent.SetWindowVisibility` (`self.Widget`) "SelfHitTestInvisible")
  (`self.OnMinigameEnd` (== AnswerIndex (`self.GoodAnswer`))))

(fn `UserConstructionScript`
  (`parent.UserConstructionScript`))