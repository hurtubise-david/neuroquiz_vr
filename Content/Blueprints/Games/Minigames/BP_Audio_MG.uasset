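; Audio minigame Blueprint that pairs a widget answer UI with a sound played in the world.
; On StartEvent it shows the widget component after a brief delay, caches its WBP_audio instance and binds the answer-chosen callback.
; It then spawns the sound at a hardcoded location and binds its finish callback.
; The answer handler is empty and the finish handler only waits, so neither has any gameplay effect.
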(event `self.StartEvent`
  (bind _returnvalue (`WidgetComponent.GetUserWidgetObject` (`self.Widget`)))
  (`KismetSystemLibrary.Delay` 0.01)
  (`WidgetComponent.SetWindowVisibility` (`self.Widget`) "Visible")
  (bind _aswbp_audio (cast `/Game/UI/WBP_audio` _returnvalue))
  (if (`KismetSystemLibrary.IsValid` _returnvalue)
    (set `self.WBP Audio` _aswbp_audio)
    (add `/Game/UI/WBP_audio.OnAnswerChosen` _aswbp_audio (delegate `AnswerChosen`))
    (bind _returnvalue_2 (`GameplayStatics.SpawnSoundAtLocation` (`self.sound`) (-20.0 400.0 30.0) (struct) 1.0 1.0 0.0 null null))
    (add `AudioComponent.OnAudioFinished` _returnvalue_2 (delegate `AudioFinished`))))

(event `AnswerChosen`
  (params (AnswerIndex :type Integer)))

(event `AudioFinished`
  (`KismetSystemLibrary.Delay` 0.2))

(fn `UserConstructionScript`
  (`parent.UserConstructionScript`))