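; Multiple-choice quiz minigame Blueprint that asks one question from a data array per start event.
; It fills a WBP_QCM widget and plays the question's sound, whose completion reveals the answers, then enables them and starts a 30-second timeout.
; Timeout ends the minigame as a failure.
; A choice clears the timer and increments Index before the reported result is evaluated, so that comparison reads the next entry.
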(event `self.StartEvent`
  (bind _widgetqcm (`self.WidgetQCM`))
  (bind _output (`|GetArrayItem` (`self.data`) (`self.index`)))
  (`KismetSystemLibrary.Delay` 0.1)
  (`WidgetComponent.SetWindowVisibility` (`self.qcm`) "Visible")
  (bind _aswbp_qcm (cast `/Game/UI/WBP_QCM` (`WidgetComponent.GetUserWidgetObject` (`self.qcm`)))
    (:`then`
      (bind _output_get (set `self.WidgetQCM` _aswbp_qcm))
      (if (`KismetSystemLibrary.IsValid` _output_get)
        (`SceneComponent.SetVisibility` (`self.qcm`) true false)
        (add `/Game/UI/WBP_QCM.OnAnswerChosen` (`self.WidgetQCM`) (delegate `OnAnswerChosen_Event`))
        (`KismetSystemLibrary.PrintString` "it works")
        (`/Game/UI/WBP_QCM.SetAnswers` _widgetqcm (`/Game/Blueprints/Games/dataAssets/BP_DataQCM.reponseTextArray` _output))
        (`/Game/UI/WBP_QCM.SetQuestion` _widgetqcm (`/Game/Blueprints/Games/dataAssets/BP_DataQCM.question` _output))
        (`/Game/UI/WBP_QCM.DisplayQuestion` _widgetqcm)
        (bind _returnvalue (`GameplayStatics.SpawnSound2D` (`/Game/Blueprints/Games/dataAssets/BP_DataQCM.sound` (`|GetArrayItem` (`self.data`) (`self.index`))) 1.0 1.0 0.0 null))
        (add `AudioComponent.OnAudioFinished` _returnvalue (delegate `OnSoundCompletedQuestion`))
        (`KismetSystemLibrary.Delay` 0.1)
        (else
          (`KismetSystemLibrary.PrintString` "CAST FAILED"))))
    (:`CastFailed`
      (`KismetSystemLibrary.PrintString` "woops"))))

(event `OnSoundCompletedQuestion`
  (bind _widgetqcm (`self.WidgetQCM`))
  (`/Game/UI/WBP_QCM.DisplayAnswers` _widgetqcm)
  ; ça serait cool avoir un son ici
  (`KismetSystemLibrary.Delay` 1.0)
  (`/Game/UI/WBP_QCM.ActivateAnswers` _widgetqcm)
  (bind _returnvalue (`KismetSystemLibrary.K2_SetTimerDelegate` (delegate `TimerEvent`) 30.0))
  (set `self.timerHandle` _returnvalue))

(event `TimerEvent`
  (`/Game/UI/WBP_QCM.HideAll` (`self.WidgetQCM`))
  (`WidgetComponent.SetWindowVisibility` (`self.qcm`) "SelfHitTestInvisible")
  (`self.OnMinigameEnd` false))

(event `OnAnswerChosen_Event`
  (params (AnswerIndex :type Integer))
  (bind _returnvalue (== AnswerIndex (`/Game/Blueprints/Games/dataAssets/BP_DataQCM.reponse` (`|GetArrayItem` (`self.data`) (`self.index`)))))
  (`KismetSystemLibrary.PrintString` "Answer nb")
  (`KismetSystemLibrary.PrintString` (`KismetStringLibrary.Conv_IntToString` AnswerIndex))
  (if _returnvalue
    (`KismetSystemLibrary.PrintString` "bonne reponse")
    (else
      (`KismetSystemLibrary.PrintString` "Mauvaise reponse")))
  (`/Game/UI/WBP_QCM.HideAll` (`self.WidgetQCM`))
  (`/Engine/EditorBlueprintResources/StandardMacros.IncrementInt` (`self.index`)
    (:`  `
      (`KismetSystemLibrary.K2_ClearAndInvalidateTimerHandle` (`self.timerHandle`))
      (`WidgetComponent.SetWindowVisibility` (`self.qcm`) "SelfHitTestInvisible")
      (`self.OnMinigameEnd` _returnvalue))))

(fn `UserConstructionScript`
  (`parent.UserConstructionScript`))