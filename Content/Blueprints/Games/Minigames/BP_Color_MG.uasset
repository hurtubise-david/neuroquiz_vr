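; Color minigame actor that presents a question through a WBP_color widget and reports win or loss via OnMinigameEnd.
; StartEvent shows the widget, binds its answer callback and plays a sound, whose finish triggers a delayed sequence of text changes before buttons appear.
; A timer then starts; choosing an answer ends the game with an Answer comparison result, while timer expiry ends it as failed, both hiding the canvas.
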(event `self.StartEvent`
  (bind _returnvalue (`WidgetComponent.GetUserWidgetObject` (`self.Widget`)))
  (`KismetSystemLibrary.Delay` 0.01)
  (`WidgetComponent.SetWindowVisibility` (`self.Widget`) "Visible")
  (bind _aswbp_color (cast `/Game/UI/WBP_color` _returnvalue))
  (if (`KismetSystemLibrary.IsValid` _returnvalue)
    (set `self.WBP` _aswbp_color)
    (add `/Game/UI/WBP_color.OnAnswerChosen` _aswbp_color (delegate `AnswerChosen`))
    (bind _returnvalue_2 (`GameplayStatics.SpawnSoundAtLocation` (`self.sound`) (-20.0 400.0 30.0) (struct) 1.0 1.0 0.0 null null))
    (add `AudioComponent.OnAudioFinished` _returnvalue_2 (delegate `AudioFinished`))))

(event `AudioFinished`
  (bind _wbp (`self.WBP`))
  (`KismetSystemLibrary.Delay` 0.2)
  (`/Game/UI/WBP_color.Show Text` (`self.WBP`) false)
  (`KismetSystemLibrary.Delay` 1.0)
  (`/Game/UI/WBP_color.HideText` _wbp)
  (`KismetSystemLibrary.Delay` 0.2)
  (`/Game/UI/WBP_color.ShowButton` _wbp)
  (bind _returnvalue (`KismetSystemLibrary.K2_SetTimerDelegate` (delegate `OnTimerEnd`)))
  (set `self.NewVar` _returnvalue))

(event `AnswerChosen`
  (params (Answer :type Integer))
  (`KismetSystemLibrary.Delay` 0.1)
  (`/Game/UI/WBP_color.hideCanvas` (`self.WBP`))
  (`WidgetComponent.SetWindowVisibility` (`self.Widget`) "SelfHitTestInvisible")
  (`self.OnMinigameEnd` (== Answer (`self.Answer`))))

(event `OnTimerEnd`
  (`/Game/UI/WBP_color.hideCanvas` (`self.WBP`))
  (`WidgetComponent.SetWindowVisibility` (`self.Widget`) "SelfHitTestInvisible")
  (`self.OnMinigameEnd` false))

(fn `UserConstructionScript`
  (`parent.UserConstructionScript`))