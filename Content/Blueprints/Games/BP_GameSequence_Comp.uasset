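; Game-show sequencer that runs a series of minigames in a VR level, then opens L_Collaboration.
; A choice widget event spawns five NPCs as allies and enemies, then starts the first minigame through its end-event dispatcher.
; Results play narration: wins add TV points and applause, losses trigger pawn stress and start the next game when audio finishes; wins have no such continuation here.
; Chained ending audio picks good or bad by points.
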(event `self.ReceiveBeginPlay`
  ; Comrade Choice
  (`KismetSystemLibrary.Delay` 0.01)
  (add `/Game/Blueprints/Games/ComradesChoice.callWidget` (`self.choix`) (delegate `GameOn`)))

(event `GameOn`
  (params (Ally1 :type Integer) (Ally2 :type Integer) (Enemy1 :type Integer) (Enemy2 :type Integer) (Enemy3 :type Integer))
  ; Spawning Comrades
  (`|SpawnActorFromClass` "/Game/Blueprints/characters/BP_Alex.BP_Alex_C" (`|GetArrayItem` (`self.NPCs`) Ally1) "Undefined" "MultiplyWithRoot" null null)
  (`|SpawnActorFromClass` "/Game/Blueprints/characters/BP_Amir.BP_Amir_C" (`|GetArrayItem` (`self.NPCs`) Ally2) "Undefined" "MultiplyWithRoot" null null)
  (`|SpawnActorFromClass` "/Game/Blueprints/characters/BP_Jess.BP_Jess_C" (`|GetArrayItem` (`self.NPCs`) Enemy1) "Undefined" "MultiplyWithRoot" null null)
  (`|SpawnActorFromClass` "/Game/Blueprints/characters/BP_Kevin.BP_Kevin_C" (`|GetArrayItem` (`self.NPCs`) Enemy2) "Undefined" "MultiplyWithRoot" null null)
  (`|SpawnActorFromClass` "/Game/Blueprints/characters/BP_Zoe.BP_Zoe_C" (`|GetArrayItem` (`self.NPCs`) Enemy3) "Undefined" "MultiplyWithRoot" null null)
  (`self.GameLoop`))

(event `GameLoop`
  (bind _output (`|GetArrayItem` (`self.minigame`) (`self.index`)))
  (add `/Game/Blueprints/Games/Minigames/BP_Minigame.OnMinigameEnd` _output (delegate `minigameEnd`))
  (`/Game/Blueprints/Games/Minigames/BP_Minigame.StartEvent` _output))

(event `CustomEvent`
  (if (< (`self.index`) (`KismetArrayLibrary.Array_Length` (`self.minigame`)))
    (bind _output (`|GetArrayItem` (`self.minigame`) (stale `minigameEnd` _result)))
    (add `/Game/Blueprints/Games/Minigames/BP_Minigame.OnMinigameEnd` _output (delegate `minigameEnd`))
    (`/Game/Blueprints/Games/Minigames/BP_Minigame.StartEvent` _output)
    (else
      (`KismetSystemLibrary.PrintString` "fin")
      (bind _returnvalue (`GameplayStatics.SpawnSoundAtLocation` "/Game/Audio/NarationV2/End1_comp.End1_comp" (-20.0 400.0 30.0) (struct) 1.0 1.0 0.0 null null))
      (add `AudioComponent.OnAudioFinished` _returnvalue (delegate `EndScene`)))))

(event `minigameEnd`
  (params (hasWon :type Boolean))
  (clear `/Game/Blueprints/Games/Minigames/BP_Minigame.OnMinigameEnd` (`|GetArrayItem` (`self.minigame`) (`self.index`)))
  (`self.OnMinigameAnswer` hasWon)
  (bind _result (`/Engine/EditorBlueprintResources/StandardMacros.IncrementInt` (`self.index`))
    (:`  `
      (`self.result` hasWon))))

(event `result`
  (params (Won :type Boolean))
  (bind _index (`self.index`))
  (if Won
    (`/Engine/EditorBlueprintResources/StandardMacros.IncrementInt` (`self.TVPoints`)
      (:`  `
        (`GameplayStatics.PlaySoundAtLocation` (`|GetArrayItem` (`self.narrationR`) _index) (-20.0 400.0 30.0) (struct) 1.0 1.0 0.0 null null null null)
        (`GameplayStatics.PlaySoundAtLocation` "/Game/Audio/Son_applaudissement.Son_applaudissement" (-20.0 400.0 30.0) (struct) 0.5 1.0 0.0 null null null null)))
    (else
      ; Player lost
      (`|ExecutionSequence`
        (:`then_0`
          (bind _returnvalue (`GameplayStatics.SpawnSound2D` (`|GetArrayItem` (`self.narrationE`) _index) 1.0 1.0 0.0 null))
          (if (`KismetSystemLibrary.IsValid` _returnvalue)
            (add `AudioComponent.OnAudioFinished` _returnvalue (delegate `CustomEvent`))
            (else
              (`self.CustomEvent`))))
        (:`then_1`
          (bind _asvrpawn (cast `/Game/VRTemplate/Blueprints/VRPawn` (`GameplayStatics.GetPlayerPawn` 0)))
          (`/Game/VRTemplate/Blueprints/VRPawn.StartStress` _asvrpawn))))))

(event `EndScene`
  (if (> (`self.TVPoints`) 0)
    (bind _returnvalue (`GameplayStatics.SpawnSoundAtLocation` "/Game/Audio/NarationV2/goodEnd_comp.goodEnd_comp" (-20.0 400.0 30.0) (struct) 1.0 1.0 0.0 null null))
    (add `AudioComponent.OnAudioFinished` _returnvalue (delegate `End2`))
    (else
      (bind _returnvalue_2 (`GameplayStatics.SpawnSoundAtLocation` "/Game/Audio/NarationV2/BadEnd_comp.BadEnd_comp" (-20.0 400.0 30.0) (struct) 1.0 1.0 0.0 null null))
      (add `AudioComponent.OnAudioFinished` _returnvalue_2 (delegate `End2`)))))

(event `End2`
  (`KismetSystemLibrary.PrintString` "END2")
  (`GameplayStatics.PlaySoundAtLocation` "/Game/Audio/NarationV2/End2_comp.End2_comp" (-20.0 400.0 30.0) (struct) 0.5 1.0 0.0 null null null null)
  (`KismetSystemLibrary.PrintString` "")
  (`GameplayStatics.OpenLevelBySoftObjectPtr` "/Game/Levels/Master/L_Collaboration.L_Collaboration"))

(fn `UserConstructionScript`)