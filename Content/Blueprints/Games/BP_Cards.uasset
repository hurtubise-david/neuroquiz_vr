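; BP_Cards is a card-placement minigame where cards must match an answer sequence of types and rotations within a two-minute limit.
; Cards stay hidden until StartGame reveals them, clears recorded placements and starts the timeout that ends the game as lost unless HasWon is set.
; OnCardPlaced records each card and, once the count matches the answer, checks types in order but only the first rotation, reporting a win on success.
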(event `ChangeCardVisibility`
  (params (isVisible :type Boolean))
  (for _array_element (`self.Cards`)
    (`SceneComponent.SetVisibility` (`Actor.RootComponent` _array_element) isVisible true)))

(event `self.ReceiveBeginPlay`
  (`self.ChangeCardVisibility` false))

(event `Initialize`
  (`self.ChangeCardVisibility` true)
  (`KismetArrayLibrary.Array_Clear` (`self.cardType`))
  (`KismetArrayLibrary.Array_Clear` (`self.cardRotation`))
  (`KismetSystemLibrary.Delay` 120.0)
  (if (not (`self.hasWon`))
    (`self.OnMinigameEnd` false)))

(event `OnCardPlaced`
  (params (cardPlaced :type "/Game/Blueprints/Logic/BP_CardInteraction Object Reference"))
  (`KismetArrayLibrary.Array_Add` (`self.cardRotation`) (`KismetMathLibrary.Conv_BoolToInt` (`/Game/Blueprints/Logic/BP_CardInteraction.bIsTwisted` cardPlaced)))
  (`KismetArrayLibrary.Array_Add` (`self.cardType`) (`/Game/Blueprints/Logic/BP_CardInteraction.cardType` cardPlaced))
  (if (== (`KismetArrayLibrary.Array_Length` (`self.cardRotation`)) (`KismetArrayLibrary.Array_Length` (`self.cardRotationAnswer`)))
    (set `self.loopFinished` true)
    (for _index (range (`KismetArrayLibrary.Array_Length` (`self.cardTypeAnswer`))) :!label _label
      (if (not (and (== (`|GetArrayItem` (`self.cardType`) _index) (`|GetArrayItem` (`self.cardTypeAnswer`) _index)) (== (`|GetArrayItem` (`self.cardRotation`)) (`|GetArrayItem` (`self.cardRotationAnswer`)))))
        (set `self.loopFinished` false)
        (`self.LoopBreak`)))
    (if (`self.loopFinished`)
      (`self.OnMinigameEnd` true))))

(event `LoopBreak`
  (goto _label :!via `Break`))

(fn `StartGame`
  (`self.Initialize`))

(fn `UserConstructionScript`
  (`parent.UserConstructionScript`))