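; BP_GameSequence_Collab runs a series of minigames in order, then moves the game on to the finale.
; It starts each entry in the Minigame array and listens for its end event before starting the next.
; Each result plays indexed win or loss narration, and wins also add to TVPoints.
; After the last minigame, an ending sound plays and its finish event loads the L_Finale level instance.
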(event `self.ReceiveBeginPlay`
  (bind _output (`|GetArrayItem` (`self.minigame`) (`self.index`)))
  (add `/Game/Blueprints/Games/Minigames/BP_Minigame.OnMinigameEnd` _output (delegate `minigameEnded`))
  (`/Game/Blueprints/Games/Minigames/BP_Minigame.StartEvent` _output))

(event `minigameEnded`
  (params (hasWon :type Boolean))
  (clear `/Game/Blueprints/Games/Minigames/BP_Minigame.OnMinigameEnd` (`|GetArrayItem` (`self.minigame`) (`self.index`)))
  (bind _result (`/Engine/EditorBlueprintResources/StandardMacros.IncrementInt` (`self.index`))
    (:`  `
      (`self.result` hasWon)
      (if (< _result (`KismetArrayLibrary.Array_Length` (`self.minigame`)))
        (bind _output (`|GetArrayItem` (`self.minigame`) _result))
        (add `/Game/Blueprints/Games/Minigames/BP_Minigame.OnMinigameEnd` _output (delegate `minigameEnded`))
        (`/Game/Blueprints/Games/Minigames/BP_Minigame.StartEvent` _output)
        (else
          (bind _returnvalue (`GameplayStatics.SpawnSoundAtLocation` "/Game/Audio/NarationV2/End_collab.End_collab" (-20.0 400.0 30.0) (struct) 1.0 1.0 0.0 null null))
          (add `AudioComponent.OnAudioFinished` _returnvalue (delegate `MoveOn`)))))))

(event `result`
  (params (Won :type Boolean))
  (bind _index (`self.index`))
  (if Won
    (`/Engine/EditorBlueprintResources/StandardMacros.IncrementInt` (`self.TVPoints`)
      (:`  `
        (`GameplayStatics.PlaySoundAtLocation` (`|GetArrayItem` (`self.narrationR`) _index) (-20.0 400.0 30.0) (struct) 1.0 1.0 0.0 null null null null)))
    (else
      ; Player lost
      (`GameplayStatics.PlaySound2D` (`|GetArrayItem` (`self.narrationE`) _index) 1.0 1.0 0.0 null null))))

(event `MoveOn`
  (`LevelStreamingDynamic.LoadLevelInstanceBySoftObjectPtr` "/Game/Levels/Master/L_Finale.L_Finale" (0.0 0.0 0.0) (struct) "" null))

(fn `UserConstructionScript`)