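; Tone test manager that runs a same-or-different pitch discrimination test over a fixed list of semitone intervals.
; Each trial plays a 440 Hz tone, then after a delay a copy shifted randomly up or down using the equal-tempered semitone ratio.
; Answers are graded only as same or different, though shift direction is recorded.
; Dispatchers signal readiness, evaluation and completion as trials advance automatically.
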(event `self.ReceiveBeginPlay`
  (set `self.SemitoneIntervals` (`|MakeArray` 8 5 0 0 2)))

(event `StartTest`
  (`AudioComponent.SetSound` (`self.AudioA`) "/Game/Audio/pure_440hz.pure_440hz")
  (`AudioComponent.SetSound` (`self.AudioB`) "/Game/Audio/pure_440hz.pure_440hz")
  (bind _output_get (set `self.CurrentInterval` (`|GetArrayItem` (`self.SemitoneIntervals`) (`self.TestIndex`))))
  (set `self.bIsSame` (== _output_get 0))
  (set `self.PitchFactor` (`KismetMathLibrary.MultiplyMultiply_FloatFloat` 1.05946 (`KismetMathLibrary.Conv_IntToDouble` (`self.CurrentInterval`))))
  (if (`self.bIsSame`)
    (set `self.PitchB` 1.0)
    (set `self.bIsHigher` false)
    (else
      (bind _output_get_2 (set `self.bIsHigher` (`KismetMathLibrary.RandomBool`)))
      (if _output_get_2
        (set `self.PitchB` (`self.PitchFactor`))
        (set `self.bIsHigher` true)
        (else
          (set `self.PitchB` (/ 1.0 (`self.PitchFactor`)))
          (set `self.bIsHigher` false)))))
  (`AudioComponent.SetPitchMultiplier` (`self.AudioA`) 1.0)
  (`AudioComponent.Play` (`self.AudioA`) 0.0)
  (`KismetSystemLibrary.Delay` (`self.DelayBetweenTones`))
  (`AudioComponent.SetPitchMultiplier` (`self.AudioB`) (`self.PitchB`))
  (`AudioComponent.Play` (`self.AudioB`) 0.0)
  (`self.OnAudioTestReady`)
  (set `self.AwaitingAnswer` true))

(event `PlayerAnswered`
  (params (Answer :type "String (by ref)"))
  (bind _testindex (`self.TestIndex`))
  (if (`self.AwaitingAnswer`)
    (if (== Answer "Same")
      (set `self.bCorrect` (`self.bIsSame`))
      (else
        (set `self.bCorrect` (not (`self.bIsSame`)))))
    (set `self.AwaitingAnswer` false)
    (`self.OnAudioAnswerEvaluated`)
    (`/Engine/EditorBlueprintResources/StandardMacros.IncrementInt` _testindex
      (:`  `
        (if (< _testindex (`KismetArrayLibrary.Array_Length` (`self.SemitoneIntervals`)))
          (`KismetSystemLibrary.Delay` (`self.DelayBetweenTones`))
          (`self.StartTest`)
          (else
            (`self.OnAudioTestEnded`)))))))

(fn `UserConstructionScript`)